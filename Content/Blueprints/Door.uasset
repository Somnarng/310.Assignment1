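; Door actor that shows an interact prompt widget while the player overlaps its trigger and slides open via an OpenDoor event.
; OpenDoor hides the prompt, disables the trigger, plays audio and moves the door by MoveVector, then closes it automatically after a short delay.
; Motion comes from MoveComponentTo on the Update of two timelines, with the trigger re-enabled after the closing move.
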(event `OpenDoor`
  (bind _door (`self.Door`))
  (`Widget.RemoveFromParent` (`self.InteractWidget`))
  (`PrimitiveComponent.SetCollisionEnabled` (`self.Trigger`) "NoCollision")
  (`AudioComponent.Play` (`self.AudioOpen`) 0.0)
  (`Timeline|Timeline`
    (:`Update`
      (`KismetSystemLibrary.MoveComponentTo` _door (`self.MoveVector`) (struct) false false 3.0)
      (`AudioComponent.Stop` (`self.AudioOpen`))
      (`KismetSystemLibrary.Delay` 1.0)
      (`AudioComponent.Play` (`self.AudioClose`) 0.0)
      (`Timeline|Timeline_0`
        (:`Update`
          (`KismetSystemLibrary.MoveComponentTo` _door)
          (`PrimitiveComponent.SetCollisionEnabled` (`self.Trigger`) "QueryOnly"))))))

(event `self.Trigger.OnComponentBeginOverlap`
  (params (OverlappedComponent :type "PrimitiveComponent Object Reference") (OtherActor :type "Actor Object Reference") (OtherComp :type "PrimitiveComponent Object Reference") (OtherBodyIndex :type Integer) (bFromSweep :type Boolean) (SweepResult :type "HitResult Structure (by ref)"))
  (if (== OtherActor (`GameplayStatics.GetPlayerCharacter` 0))
    (`UserWidget.AddToViewport` (`self.InteractWidget`) 0)))

(event `self.Trigger.OnComponentEndOverlap`
  (params (OverlappedComponent :type "PrimitiveComponent Object Reference") (OtherActor :type "Actor Object Reference") (OtherComp :type "PrimitiveComponent Object Reference") (OtherBodyIndex :type Integer))
  (if (== (`GameplayStatics.GetPlayerCharacter` 0) OtherActor)
    (`Widget.RemoveFromParent` (`self.InteractWidget`))))

(event `self.ReceiveBeginPlay`
  (bind _returnvalue (`|CreateWidget` "/Game/Blueprints/P_Interact.P_Interact_C"))
  (set `self.InteractWidget` _returnvalue))

(fn `UserConstructionScript`)